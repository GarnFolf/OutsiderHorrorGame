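; Actor component for a grid inventory of shaped, rotatable, stackable items, with Tab toggling the inventory widget.
; Items are stored by anchor cell in Inventory, while InventoryState maps each grid cell to occupied or free.
; Pickups top up matching stacks, then search for free space in four rotations, returning any unplaced remainder to the world item.
; Drops spawn a placeholder item where a downward trace ahead of the owner hits.
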(event EventBeginPlay
  (State|DefaultInventoryState))

(event Input|KeyboardEvents|Tab
  (params (Key :type Key%20Structure))
  (bind _returnvalue (Game|GetPlayerCharacter 0))
  (bind _returnvalue_2 (Game|GetPlayerCharacter 0))
  (bind _playerstate (Variables|/Script/Engine.Pawn|GetPlayerState _returnvalue_2))
  (bind _playerstate_2 (Variables|/Script/Engine.Pawn|GetPlayerState _returnvalue))
  (bind _returnvalue_3 (Game|GetPlayerController _playerstate))
  (bind _returnvalue_4 (Game|GetPlayerController _playerstate_2))
  (:Pressed
    (Variables|Default|GetAs%20UMG_Inventory
      (:then
        (Widget|RemovefromParent (Variables|Default|GetAs%20UMG_Inventory))
        (Variables|Default|SetAs%20UMG_Inventory 0)
        (Variables|/Script/Engine.PlayerController|SetbShowMouseCursor _returnvalue_4 false)
        (Input|SetInputModeGameOnly _returnvalue_4 false))
      (:else
        (bind _returnvalue_5 (UserInterface|CreateWidget "/Game/Elijah/Inventory/Widget/UMG_Inventory.UMG_Inventory_C"))
        (bind _output_get (Variables|Default|SetAs%20UMG_Inventory _returnvalue_5))
        (UserInterface|Viewport|AddtoViewport _output_get 0)
        (Variables|/Script/Engine.PlayerController|SetbShowMouseCursor _returnvalue_3 false)
        (Input|SetInputModeGameandUI _returnvalue_3 0 "DoNotLock" true false)))))

(fn DefaultInventoryState
  (for _index (range 0 (- (Variables|Default|GetInventorySize) 1))
    (Utilities|Map|Add (Variables|Default|GetInventoryState) (Math|Vector2D|MakeVector2D (LocalVariables|GetL-GridX) (LocalVariables|GetL-GridY)) false)
    (if (== (LocalVariables|GetL-GridX) (- (Variables|Default|GetInventoryWidth) 1))
      (LocalVariables|SetL-GridX 0.0)
      (Math|Float|IncrementFloat (LocalVariables|GetL-GridY))
      (else
        (Math|Float|IncrementFloat (LocalVariables|GetL-GridX)))))
  (bind _keys (Utilities|Map|Keys (Variables|Default|GetInventory)))
  (for _array_element _keys
    (State|AddtoState (.Value (Utilities|Map|Find (Variables|Default|GetInventory) _array_element)) _array_element)))

(fn AddtoState
  (params (ST_Item :type ST%20Item%20Structure%20%28by%20ref%29) (Location :type Vector%202D%20Structure))
  (bind (_dataasset _rotation) (Utilities|Struct|BreakST_Item ST_Item))
  (bind _defaultshape (Default|GetShape _dataasset _rotation))
  (for _array_element _defaultshape
    (Utilities|Map|Add (Variables|Default|GetInventoryState) (+ _array_element Location) true)
    (return)))

(fn RemovefromState
  (params (ST_Item :type ST%20Item%20Structure%20%28by%20ref%29) (Location :type Vector%202D%20Structure))
  (bind (_dataasset _rotation) (Utilities|Struct|BreakST_Item ST_Item))
  (bind _defaultshape (Default|GetShape _dataasset _rotation))
  (for _array_element _defaultshape
    (Utilities|Map|Add (Variables|Default|GetInventoryState) (+ _array_element Location) false)))

(fn AddtoInventory
  (params (Key :type Vector%202D%20Structure%20%28by%20ref%29) (Value :type ST%20Item%20Structure%20%28by%20ref%29) (ModifyState :type Boolean))
  (Utilities|Map|Add (Variables|Default|GetInventory) Key Value)
  (if ModifyState
    (State|AddtoState Value Key)
    (return)))

(fn RemovefromInventory
  (params (Key :type Vector%202D%20Structure) (Modify%20State :type Boolean))
  (Utilities|FlowControl|Sequence
    (:then_0
      (if Modify%20State
        (State|RemovefromState (.Value (Utilities|Map|Find (Variables|Default|GetInventory) Key)) Key)))
    (:then_1
      (Utilities|Map|Remove (Variables|Default|GetInventory) Key))))

(fn IsNotFullyStacked
  (params (ItemStructure :type ST%20Item%20Structure))
  (bind (_dataasset _rotation _quantity) (Utilities|Struct|BreakST_Item ItemStructure))
  (bind _maxquantity (Variables|/Game/Elijah/Inventory/Data/DataAsset_Items.DataAsset_Items_C|GetMaxQuantity _dataasset))
  (return (> _maxquantity _quantity) (- _maxquantity _quantity)))

(fn WhereShapeFits
  (params (Shape :type Array%20of%20Vector%202D%20Structures))
  (bind _keys (Utilities|Map|Keys (Variables|Default|GetInventoryState)))
  (for _array_element _keys
    (if (.ReturnValue (Utilities|Map|Find (Variables|Default|GetInventoryState) (- _array_element (Utilities|Array|Get(acopy) Shape))))
      (if (not (.Value (Utilities|Map|Find (Variables|Default|GetInventoryState) (- _array_element (Utilities|Array|Get(acopy) Shape)))))
        (LocalVariables|SetL-EmptySlot _array_element)
        (bind _array_element_2 (Utilities|Array|ForEachLoopwithBreak Shape :!label _label)
          (:LoopBody
            (if (or (.Value (Utilities|Map|Find (Variables|Default|GetInventoryState) (+ (LocalVariables|GetL-EmptySlot) _array_element_2))) (not (.ReturnValue (Utilities|Map|Find (Variables|Default|GetInventoryState) (+ (LocalVariables|GetL-EmptySlot) _array_element_2)))))
              (LocalVariables|SetL-Failed true)
              (goto _label Break)))
          (:Completed
            (if (LocalVariables|GetL-Failed)
              (LocalVariables|SetL-Failed false)
              (else
                (return true (LocalVariables|GetL-EmptySlot)))))))))
  (return false ""))

(fn PickupItem
  (params (ItemRef :type Placeholer%20Item%20Object%20Reference))
  (bind _remaining (Manage|AddItemfromFloor (Variables|/Game/Elijah/Inventory/Items/placeholer_Item.placeholer_Item_C|GetItemStructure ItemRef)))
  (if (== _remaining 0)
    (return true)
    (else
      (Default|ModifyQuantity ItemRef _remaining)
      (return false))))

(fn CheckRotationFit
  (params (InputPin :type ST%20Item%20Structure) (InputPin2 :type Float%20%28double-precision%29))
  (bind (_dataasset _rotation _quantity) (Utilities|Struct|BreakST_Item InputPin))
  (bind _defaultshape (Default|GetShape (Utilities|Struct|BreakST_Item InputPin) InputPin2))
  (bind (_returnvalue _validkey) (Conditions|WhereShapeFits _defaultshape))
  (if _returnvalue
    (Inventory|AddtoInventory _validkey (Utilities|Struct|MakeST_Item _dataasset InputPin2 _quantity) true)
    (return true)
    (else
      (return false))))

(fn AddItemfromFloor
  (params (Item%20Structure :type ST%20Item%20Structure))
  (LocalVariables|SetL-ItemStruct Item%20Structure)
  (Utilities|FlowControl|Sequence
    (:then_0
      (bind _keys (Utilities|Map|Keys (Variables|Default|GetInventory)))
      (for _array_element _keys
        (bind _output_get (LocalVariables|SetL-LoopKey _array_element))
        (LocalVariables|SetL-LoopValue (.Value (Utilities|Map|Find (Variables|Default|GetInventory) _output_get)))
        (if (== (Utilities|Struct|BreakST_Item (LocalVariables|GetL-ItemStruct)) (Utilities|Struct|BreakST_Item (LocalVariables|GetL-LoopValue)))
          (bind (_returnvalue _remaining) (Conditions|IsNotFullyStacked (LocalVariables|GetL-LoopValue)))
          (if _returnvalue
            (Inventory|AddtoInventory (LocalVariables|GetL-LoopKey) (Utilities|Struct|MakeST_Item (.DataAsset (Utilities|Struct|BreakST_Item (LocalVariables|GetL-LoopValue))) (.Rotation (Utilities|Struct|BreakST_Item (LocalVariables|GetL-LoopValue))) (Math|Integer|Clamp(Integer) (+ (.Quantity (Utilities|Struct|BreakST_Item (LocalVariables|GetL-LoopValue))) (Utilities|Struct|BreakST_Item (LocalVariables|GetL-ItemStruct))) 0 (Variables|/Game/Elijah/Inventory/Data/DataAsset_Items.DataAsset_Items_C|GetMaxQuantity (.DataAsset (Utilities|Struct|BreakST_Item (LocalVariables|GetL-LoopValue)))))) false)
            (bind _structout (Utilities|Struct|SetmembersinST_Item (LocalVariables|GetL-ItemStruct) (- (Utilities|Struct|BreakST_Item (LocalVariables|GetL-ItemStruct)) _remaining)))
            (if (<= (Utilities|Struct|BreakST_Item _structout) 0)
              (return true 0))))))
    (:then_1
      (Utilities|FlowControl|Sequence
        (:then_0
          (bind _sucsess (Manage|CheckRotationFit (LocalVariables|GetL-ItemStruct) 0.0))
          (if _sucsess
            (return true 0)))
        (:then_1
          (bind _sucsess_2 (Manage|CheckRotationFit (LocalVariables|GetL-ItemStruct) 9e+01))
          (if _sucsess_2
            (return true 0)))
        (:then_2
          (bind _sucsess_3 (Manage|CheckRotationFit (LocalVariables|GetL-ItemStruct) 1.8e+02))
          (if _sucsess_3
            (return true 0)))
        (:then_3
          (bind _sucsess_4 (Manage|CheckRotationFit (LocalVariables|GetL-ItemStruct) -9e+01))
          (if _sucsess_4
            (return true 0)))
        (:then_4
          (return false (Utilities|Struct|BreakST_Item (LocalVariables|GetL-ItemStruct))))))))

(fn DropItem
  (params (Structure :type ST%20Item%20Structure))
  (bind _returnvalue (Components|GetOwner))
  (bind _returnvalue_2 (Transformation|GetActorLocation _returnvalue))
  (bind _returnvalue_3 (Transformation|GetActorForwardVector _returnvalue))
  (bind _returnvalue_4 (* _returnvalue_3 6e+02))
  (bind _returnvalue_5 (+ _returnvalue_2 _returnvalue_4))
  (bind (_outhit _returnvalue_6) (Collision|LineTraceByChannel _returnvalue_5 (- _returnvalue_5 "0.000000,0.000000,500.000000") "TraceTypeQuery1" false 0 "None"))
  (if _returnvalue_6
    (Game|SpawnActorfromClass "/Game/Elijah/Inventory/Items/placeholer_Item.placeholer_Item_C" (Math|Conversions|ToTransform(Vector) (.ImpactPoint (Collision|BreakHitResult _outhit))) "Undefined" "MultiplyWithRoot" 0 Structure 0)))